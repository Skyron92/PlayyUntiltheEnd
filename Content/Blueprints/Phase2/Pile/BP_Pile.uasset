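; Addition puzzle actor where the player picks how many cells to add to a random count of green piles to reach a displayed total.
; SelectPile parses the number from the clicked name and lights that many Cal cells green.
; Verify animates a button press via Timeline, then checks the sum.
; Success notifies BP_GameInstance and destroys the actor; failure flashes red, reports it and rerolls the question.
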(event `self.ReceiveBeginPlay`
  (`self.f_ChargeList`)
  (`self.RechargeCalculation`)
  (set `self.ButtonLocation` (`SceneComponent.K2_GetComponentLocation` (`self.Cylinder`))))

(event `RechargeCalculation`
  ;[1 0.8104 0] Recommencer la question
  (for _array_element (`self.ListPiles`)
    (`PrimitiveComponent.SetMaterial` _array_element 0 "/Engine/BasicShapes/BasicShapeMaterial.BasicShapeMaterial"))
  (for _array_element_2 (`self.ListCal`)
    (`PrimitiveComponent.SetMaterial` _array_element_2 0 "/Engine/BasicShapes/BasicShapeMaterial.BasicShapeMaterial"))
  (bind _output_get (set `self.StartPile` (`KismetMathLibrary.RandomIntegerInRange` 1 10)))
  (set `self.NumberInital` (+ _output_get (`KismetMathLibrary.RandomIntegerInRange` 1 10)))
  (`self.f_SetUpPiles` (`self.StartPile`))
  (`TextRenderComponent.K2_SetText` (`self.w`) (`KismetTextLibrary.Conv_IntToText` (`self.NumberInital`))))

(event `SelectPile`
  (params (Name :type String))
  (bind _returnvalue (`KismetStringLibrary.Conv_StringToInt` (`KismetStringLibrary.GetSubstring` Name 3 2)))
  ;[0.02606 1 0] Joueur à selectionner la réponse
  (for _array_element (`self.ListCal`)
    (`PrimitiveComponent.SetMaterial` _array_element 0 "/Engine/BasicShapes/BasicShapeMaterial.BasicShapeMaterial")
    (set `self.Calculation` _returnvalue)
    (`self.f_SetUpCals` _returnvalue)))

(event `Verify`
  (bind (_buttonlocation_x _buttonlocation_y _buttonlocation_z) (`KismetMathLibrary.BreakVector` (`self.ButtonLocation`)))
  (bind _asbp_game_instance (cast `/Game/Blueprints/Quest/BP_GameInstance` (`GameplayStatics.GetGameInstance`) :!pure true))
  ;[0.8965 1 0.3595] Vérifier la réponse
  (bind (_direction _buttonmovement) (`Timeline|Timeline` :!via `PlayFromStart`)
    (:`Update`
      (`SceneComponent.K2_SetWorldLocation` (`self.Cylinder`) (`KismetMathLibrary.MakeVector` _buttonlocation_x _buttonlocation_y (`KismetMathLibrary.Lerp` _buttonlocation_z (- _buttonlocation_z 5.0) _buttonmovement)) false false))
    (:`Finished`
      (if (== (+ (`self.Calculation`) (`self.StartPile`)) (`self.NumberInital`))
        (`/Game/Blueprints/Quest/BP_GameInstance.f_EndQuestCal` _asbp_game_instance)
        (`KismetSystemLibrary.Delay` 3.0)
        (`self.K2_DestroyActor`)
        (else
          (`self.f_Erreur` (`self.Calculation`))
          (`/Game/Blueprints/Quest/BP_GameInstance.f_QuestFailed` _asbp_game_instance)
          (`KismetSystemLibrary.Delay` 0.2)
          (`self.RechargeCalculation`))))))

(fn `f_ChargeList`
  (bind _listcal (`self.ListCal`))
  (bind _listpiles (`self.ListPiles`))
  (`KismetArrayLibrary.Array_Add` _listpiles (`self.Pile`))
  (`KismetArrayLibrary.Array_Add` _listpiles (`self.Pile2`))
  (`KismetArrayLibrary.Array_Add` _listpiles (`self.Pile3`))
  (`KismetArrayLibrary.Array_Add` _listpiles (`self.Pile4`))
  (`KismetArrayLibrary.Array_Add` _listpiles (`self.Pile5`))
  (`KismetArrayLibrary.Array_Add` _listpiles (`self.Pile6`))
  (`KismetArrayLibrary.Array_Add` _listpiles (`self.Pile7`))
  (`KismetArrayLibrary.Array_Add` _listpiles (`self.Pile8`))
  (`KismetArrayLibrary.Array_Add` _listpiles (`self.Pile9`))
  (`KismetArrayLibrary.Array_Add` _listpiles (`self.Pile10`))
  (`KismetArrayLibrary.Array_Add` _listcal (`self.Cal1`))
  (`KismetArrayLibrary.Array_Add` _listcal (`self.Cal2`))
  (`KismetArrayLibrary.Array_Add` _listcal (`self.Cal3`))
  (`KismetArrayLibrary.Array_Add` _listcal (`self.Cal4`))
  (`KismetArrayLibrary.Array_Add` _listcal (`self.Cal5`))
  (`KismetArrayLibrary.Array_Add` _listcal (`self.Cal6`))
  (`KismetArrayLibrary.Array_Add` _listcal (`self.Cal7`))
  (`KismetArrayLibrary.Array_Add` _listcal (`self.Cal8`))
  (`KismetArrayLibrary.Array_Add` _listcal (`self.Cal9`))
  (`KismetArrayLibrary.Array_Add` _listcal (`self.Cal10`)))

(fn `f_Erreur`
  (params (NumberOfCal :type Integer))
  (locals (Index :type Integer) (Limite :type Integer))
  (set `local.Limite` NumberOfCal)
  (bind _output_get (set `local.Index` 0))
  (while (< _output_get (`local.Limite`))
    (`PrimitiveComponent.SetMaterial` (`|GetArrayItem` (`self.ListCal`) (`local.Index`)) 0 "/AnimationSharing/AnimSharingRed.AnimSharingRed")
    (`/Engine/EditorBlueprintResources/StandardMacros.IncrementInt` (`local.Index`))))

(fn `f_SetUpCals`
  (params (NumberOfCal :type Integer))
  (locals (Index :type Integer) (Limite :type Integer))
  (set `local.Limite` NumberOfCal)
  (bind _output_get (set `local.Index` 0))
  (while (< _output_get (`local.Limite`))
    (`PrimitiveComponent.SetMaterial` (`|GetArrayItem` (`self.ListCal`) (`local.Index`)) 0 "/AnimationSharing/AnimSharingGreen.AnimSharingGreen")
    (`/Engine/EditorBlueprintResources/StandardMacros.IncrementInt` (`local.Index`))))

(fn `f_SetUpPiles`
  (params (NumberOfPile :type Integer))
  (locals (Index :type Integer) (Limite :type Integer))
  (set `local.Limite` NumberOfPile)
  (bind _output_get (set `local.Index` 0))
  (while (< _output_get (`local.Limite`))
    (`PrimitiveComponent.SetMaterial` (`|GetArrayItem` (`self.ListPiles`) (`local.Index`)) 0 "/AnimationSharing/AnimSharingGreen.AnimSharingGreen")
    (`/Engine/EditorBlueprintResources/StandardMacros.IncrementInt` (`local.Index`)))
  (set `self.SetUp` true))

(fn `UserConstructionScript`)