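; BP_Simon is a Simon-style light game piece that plays a fixed color sequence when play begins.
; After a short delay it lights the Blue, Yellow and Green meshes in turn by swapping each to its lit material, then restoring the plain one.
; The sequence is a hardcoded chain of delays that runs once, with no input handling or randomization in this Blueprint.
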(event `self.ReceiveBeginPlay`
  (bind _blue (`self.Blue`))
  (bind _yellow (`self.Yellow`))
  (bind _green (`self.Green`))
  (`KismetSystemLibrary.Delay` 1.0)
  (`PrimitiveComponent.SetMaterial` _blue 0 "/Game/Materials/M_BlueLight.M_BlueLight")
  (`KismetSystemLibrary.Delay` 1.5)
  (`PrimitiveComponent.SetMaterial` _blue 0 "/Game/Materials/M_Blue.M_Blue")
  (`PrimitiveComponent.SetMaterial` _yellow 0 "/Game/Materials/M_YellowLight.M_YellowLight")
  (`KismetSystemLibrary.Delay` 1.5)
  (`PrimitiveComponent.SetMaterial` _yellow 0 "/Game/Materials/M_Yellow.M_Yellow")
  (`PrimitiveComponent.SetMaterial` _green 0 "/Game/Materials/M_GreenLight.M_GreenLight")
  (`KismetSystemLibrary.Delay` 1.5)
  (`PrimitiveComponent.SetMaterial` _green 0 "/Game/Materials/M_Green.M_Green"))

(fn `UserConstructionScript`)