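; Timing quick-time event actor where a pointer oscillates vertically and the player tries to stop on a red zone.
; Tick moves the pointer by a fixed per-frame offset, flipping direction at upper and lower marker components, and BeginPlay shows the mouse cursor.
; DoesAction, with no caller here, checks the pointer's height against the red bounds, showing a quest-complete widget inside or quest-failed plus great sparks outside.
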(event `self.ReceiveBeginPlay`
  ;[0.218 1 0.1327] Show mouse cursor
  (set `PlayerController.bShowMouseCursor` true (`GameplayStatics.GetPlayerController` 0)))

(event `self.ReceiveTick`
  (params (DeltaSeconds :type "Float (single-precision)"))
  ;[0.3915 0.6142 1] Up-Down movement
  (`SceneComponent.K2_AddLocalOffset` (`self.Pointeur`) (`KismetMathLibrary.MakeVector` 0.0 0.0 (`self.Vitesse`)) false false)
  (bind _hasreachedthelimit (`self.HasReachTheLimit` true))
  (if _hasreachedthelimit
    (set `self.Vitesse` -1.0)
    (else
      (bind _hasreachedthelimit_2 (`self.HasReachTheLimit` false))
      (if _hasreachedthelimit_2
        (set `self.Vitesse` 1.0)))))

(event `self.GreatSpakles.OnSystemFinished`
  (params (PSystem :type "NiagaraComponent Object Reference"))
  (`SceneComponent.SetVisibility` PSystem false false))

(fn `DoesAction`
  (bind _is_in_the_red_area (`self.IsInTheReadArea`))
  (if _is_in_the_red_area
    (`SceneComponent.SetVisibility` (`self.Sparkles`) false false)
    (bind _returnvalue (`|CreateWidget` "/Game/UI/WB_QuestComplete.WB_QuestComplete_C"))
    (`UserWidget.AddToViewport` _returnvalue 0)
    (else
      (`SceneComponent.SetVisibility` (`self.Sparkles`) false false)
      (`SceneComponent.SetVisibility` (`self.GreatSpakles`) true false)
      (bind _returnvalue_2 (`|CreateWidget` "/Game/UI/WB_QuestFailed.WB_QuestFailed_C"))
      (`UserWidget.AddToViewport` _returnvalue_2 0))))

(fn `HasReachTheLimit`
  (params (`To the top` :type Boolean))
  (returns (HasReachedTheLimit :type Boolean))
  (bind (_returnvalue_x _returnvalue_y _returnvalue_z) (`KismetMathLibrary.BreakVector` (`SceneComponent.K2_GetComponentLocation` (`self.UpPoint`))))
  (bind (_returnvalue_x_2 _returnvalue_y_2 _returnvalue_z_2) (`KismetMathLibrary.BreakVector` (`SceneComponent.K2_GetComponentLocation` (`self.DownPoint`))))
  (bind (_returnvalue_x_3 _returnvalue_y_3 _returnvalue_z_3) (`KismetMathLibrary.BreakVector` (`SceneComponent.K2_GetComponentLocation` (`self.Pointeur`))))
  (if `To the top`
    (return (>= _returnvalue_z_3 _returnvalue_z))
    (else
      (return (<= _returnvalue_z_3 _returnvalue_z_2)))))

(fn `IsInTheReadArea`
  (returns (`Is in the red area` :type Boolean))
  (bind (_returnvalue_x _returnvalue_y _returnvalue_z) (`KismetMathLibrary.BreakVector` (`SceneComponent.K2_GetComponentLocation` (`self.Pointeur`))))
  (bind (_returnvalue_x_2 _returnvalue_y_2 _returnvalue_z_2) (`KismetMathLibrary.BreakVector` (`SceneComponent.K2_GetComponentLocation` (`self.BottomRed`))))
  (bind (_returnvalue_x_3 _returnvalue_y_3 _returnvalue_z_3) (`KismetMathLibrary.BreakVector` (`SceneComponent.K2_GetComponentLocation` (`self.TopRed`))))
  (return (and (>= _returnvalue_z _returnvalue_z_2) (<= _returnvalue_z _returnvalue_z_3))))

(fn `UserConstructionScript`)