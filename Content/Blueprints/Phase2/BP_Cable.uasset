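; BP_Cable is a cable the player can pick up and plug into actors tagged "Socket".
; While the player is inside its Box, GetCable is bound to the character's Interact event.
; Interacting attaches the cable end to the player, then a second press traces from the camera to connect or release it.
; Leaving the Box drops an unconnected cable and unbinds all Interact events.
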(event `self.ReceiveBeginPlay`)

(event `self.Box.OnComponentBeginOverlap`
  (params (OverlappedComponent :type "PrimitiveComponent Object Reference") (OtherActor :type "Actor Object Reference") (OtherComp :type "PrimitiveComponent Object Reference") (OtherBodyIndex :type Integer) (bFromSweep :type Boolean) (SweepResult :type "HitResult Structure (by ref)"))
  ;[0.4586 0.2657 1] Detecter si le joueur est assez proche à interagir
  (if (== (`GameplayStatics.GetPlayerCharacter` 0) OtherActor)
    (add `/Game/FirstPerson/Blueprints/BP_FirstPersonCharacter.Interact` (cast `/Game/FirstPerson/Blueprints/BP_FirstPersonCharacter` (`GameplayStatics.GetPlayerPawn` 0) :!pure true) (delegate `GetCable`))))

(event `GetCable`
  (bind _returnvalue (`GameplayStatics.GetPlayerController` 0))
  (bind _returnvalue_2 (`PlayerCameraManager.GetCameraLocation` (`PlayerController.PlayerCameraManager` _returnvalue)))
  ;[0.1567 0.2712 1] Prendre le cable
  (set `self.Connected` false)
  (if (`self.Grab`)
    (bind (_outhit _returnvalue_3) (`KismetSystemLibrary.LineTraceSingle` :`Start` _returnvalue_2 :`End` (+ _returnvalue_2 (* (`self.GetActorForwardVector` _returnvalue) 1000.0)) :`TraceChannel` "TraceTypeQuery1" :`DrawDebugType` "Persistent"))
    (if _returnvalue_3
      (bind (_bblockinghit _binitialoverlap _time _distance _location _impactpoint _normal _impactnormal _physmat _hitactor) (`GameplayStatics.BreakHitResult` _outhit))
      (if (`self.ActorHasTag` _hitactor "Socket")
        (`CableComponent.SetAttachEndTo` (`self.Cable`) _hitactor "Center" "None")
        (set `self.Grab` false)
        (set `self.Connected` true)
        (else
          (set `CableComponent.bAttachEnd` false (`self.Cable`) :!label _label)
          (set `self.Grab` false)))
      (else
        (goto _label)))
    (else
      (set `CableComponent.bAttachEnd` true (`self.Cable`))
      (`CableComponent.SetAttachEndTo` (`self.Cable`) (`GameplayStatics.GetPlayerPawn` 0) "None" "hand_lSocket")
      (set `self.Grab` true))))

(event `self.Box.OnComponentEndOverlap`
  (params (OverlappedComponent :type "PrimitiveComponent Object Reference") (OtherActor :type "Actor Object Reference") (OtherComp :type "PrimitiveComponent Object Reference") (OtherBodyIndex :type Integer))
  ;[0.4586 0.2657 1] Detecter si le joueur est assez proche à interagir
  (if (== (`GameplayStatics.GetPlayerCharacter` 0) OtherActor)
    (if (not (`self.Connected`))
      (set `CableComponent.bAttachEnd` false (`self.Cable`))
      (set `self.Grab` false))
    (clear `/Game/FirstPerson/Blueprints/BP_FirstPersonCharacter.Interact` (cast `/Game/FirstPerson/Blueprints/BP_FirstPersonCharacter` (`GameplayStatics.GetPlayerPawn` 0) :!pure true))))

(fn `UserConstructionScript`)