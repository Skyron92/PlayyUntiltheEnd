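; Cable-matching puzzle actor where the player plugs four colored cables into same-colored sockets to finish a quest.
; BeginPlay shuffles colors onto cables and sockets; GetCable attaches the chosen cable end to the player's hand.
; Release sphere-traces along the mouse direction to plug or drop it, as does leaving the Box, and matches are checked by material name.
; Four correct matches end the GameInstance quest and destroy the actor after a delay.
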(event `self.ReceiveBeginPlay`
  (bind _asbp_game_instance (cast `/Game/Blueprints/Quest/BP_GameInstance` (`GameplayStatics.GetGameInstance`)))
  (set `self.As BP Game Instance` _asbp_game_instance)
  (set `self.Normal` (`PrimitiveComponent.GetMaterial` (`self.Cube3`) 0))
  (bind _returnvalue (`KismetMaterialLibrary.CreateDynamicMaterialInstance` "/Engine/VREditor/BasicMeshes/MI_Cube_02.MI_Cube_02"))
  (set `self.Interacting` _returnvalue)
  (`self.f_GenerateRandomColors`)
  (`self.f_ChargeCableList`)
  (`self.f_ChargeSocketList`)
  (`self.RechargeColor`))

(event `GetCable`
  (params (Name :type String))
  (bind _selectedcable (`self.SelectedCable`))
  ;[0.1567 0.2712 1] Prendre le cable
  (`self.f_TakeCable` Name)
  (`GameplayStatics.PlaySound2D` "/Game/SoundDesign/Global/SoundCue/SC_Click.SC_Click" 1.0 1.0 0.0 null null)
  (`CableComponent.SetAttachEndToComponent` _selectedcable null "None")
  (set `self.Connected` false)
  (`/Engine/EditorBlueprintResources/StandardMacros.IsValid` _selectedcable
    (:`Is Valid`
      (set `CableComponent.bAttachEnd` true _selectedcable)
      (`CableComponent.SetAttachEndTo` (`self.SelectedCable`) (`GameplayStatics.GetPlayerPawn` 0) "None" "hand_lSocket")
      (if (`self.Correct`)
        (`/Game/Blueprints/Quest/BP_GameInstance.f_UpdateQuestCable` (`self.As BP Game Instance`) -1)
        (set `self.Correct` false)))))

(event `Release`
  (bind _returnvalue (`GameplayStatics.GetPlayerController` 0))
  (bind _selectedcube (`self.SelectedCube`))
  (bind _returnvalue_2 (`PlayerCameraManager.GetCameraLocation` (`PlayerController.PlayerCameraManager` _returnvalue)))
  ;[0.4586 0.2657 1] Relâcher le cable
  (`/Engine/EditorBlueprintResources/StandardMacros.IsValid` _selectedcube
    (:`Is Valid`
      (`PrimitiveComponent.SetMaterial` _selectedcube 0 (`self.Normal`))
      (set `self.SelectedCube` null)
      (bind (_outhit _returnvalue_3) (`KismetSystemLibrary.SphereTraceSingle` :`Start` _returnvalue_2 :`End` (+ _returnvalue_2 (* (`.WorldDirection` (`PlayerController.DeprojectMousePositionToWorld` _returnvalue)) 100000.0)) :`Radius` 10.0 :`TraceChannel` "TraceTypeQuery1" :`bIgnoreSelf` false))
      (if _returnvalue_3
        (bind (_bblockinghit _binitialoverlap _time _distance _location _impactpoint _normal _impactnormal _physmat _hitactor _hitcomponent) (`GameplayStatics.BreakHitResult` _outhit))
        (if (`ActorComponent.ComponentHasTag` _hitcomponent "Socket")
          (`self.f_Connect` _hitactor (`KismetSystemLibrary.GetObjectName` _hitcomponent))
          (set `self.Connected` true)
          (`GameplayStatics.PlaySound2D` "/Game/SoundDesign/Phase2/SoundCue/SC_CablePlugGood.SC_CablePlugGood" 1.0 1.0 0.0 null null)
          (set `self.SelectedCable` null)
          (if (== (`BlueprintMapLibrary.Map_Length` (`self.MapCorrectSocket`)) 4)
            (`/Game/Blueprints/Quest/BP_GameInstance.f_EndQuestCable` (`self.As BP Game Instance`))
            (`GameplayStatics.PlaySound2D` "/Game/SoundDesign/Phase1/SoundCue/SC_Win.SC_Win" 1.0 1.0 0.0 null null)
            (`KismetSystemLibrary.Delay` 3.0)
            (`self.K2_DestroyActor`))
          (else
            (set `CableComponent.bAttachEnd` false (`self.SelectedCable`) :!label _label)
            (set `self.SelectedCable` null)))
        (else
          (goto _label))))))

(event `self.Box.OnComponentEndOverlap`
  (params (OverlappedComponent :type "PrimitiveComponent Object Reference") (OtherActor :type "Actor Object Reference") (OtherComp :type "PrimitiveComponent Object Reference") (OtherBodyIndex :type Integer))
  (if (== OtherActor (`GameplayStatics.GetPlayerCharacter` 0))
    (if (not (`self.Connected`))
      (`self.Release`))))

(event `RechargeColor`
  (bind _listcolors (`self.ListColors`))
  (`KismetSystemLibrary.PrintString` (`KismetStringLibrary.Conv_IntToString` (`KismetArrayLibrary.Array_Length` _listcolors)))
  (for (_array_element _array_index) _listcolors
    (`self.f_RandomCable` _array_element _array_index))
  (`self.f_GenerateRandomColors`)
  (for (_array_element_2 _array_index_2) (`self.ListColors`)
    (`self.f_RandomSocket` _array_element_2 _array_index_2)))

(fn `f_ChargeCableList`
  (bind _listcables (`self.ListCables`))
  (`KismetArrayLibrary.Array_Add` _listcables (`self.Cable1`))
  (`KismetArrayLibrary.Array_Add` _listcables (`self.Cable2`))
  (`KismetArrayLibrary.Array_Add` _listcables (`self.Cable3`))
  (`KismetArrayLibrary.Array_Add` _listcables (`self.Cable4`)))

(fn `f_ChargeSocketList`
  (locals (NewLocalVar :type "StaticMeshComponent Object Reference"))
  (bind _listsockets (`self.ListSockets`))
  (`KismetArrayLibrary.Array_Add` _listsockets (`self.Socket1`))
  (`KismetArrayLibrary.Array_Add` _listsockets (`self.Socket2`))
  (`KismetArrayLibrary.Array_Add` _listsockets (`self.Socket3`))
  (`KismetArrayLibrary.Array_Add` _listsockets (`self.Socket4`)))

(fn `f_Connect`
  (params (Actor :type "Actor Object Reference") (Selection :type String))
  (bind _selectedcable (`self.SelectedCable`))
  (switch `string` Selection
    (:`Socket1`
      (`CableComponent.SetAttachEndToComponent` _selectedcable (`self.Center1`) "None")
      (if (`KismetStringLibrary.EqualEqual_StrStr` (`KismetSystemLibrary.GetObjectName` (`PrimitiveComponent.GetMaterial` (`self.SelectedCable`) 0)) (`KismetSystemLibrary.GetObjectName` (`PrimitiveComponent.GetMaterial` (`self.Socket1`) 0)))
        (`BlueprintMapLibrary.Map_Add` (`self.MapCorrectSocket`) (`KismetStringLibrary.Conv_StringToInt` (`KismetStringLibrary.GetSubstring` (`KismetSystemLibrary.GetObjectName` (`self.SelectedCable`)) 5)) 1)))
    (:`Socket2`
      (`CableComponent.SetAttachEndToComponent` _selectedcable (`self.Center2`) "None")
      (if (`KismetStringLibrary.EqualEqual_StrStr` (`KismetSystemLibrary.GetObjectName` (`PrimitiveComponent.GetMaterial` (`self.SelectedCable`) 0)) (`KismetSystemLibrary.GetObjectName` (`PrimitiveComponent.GetMaterial` (`self.Socket2`) 0)))
        (`BlueprintMapLibrary.Map_Add` (`self.MapCorrectSocket`) (`KismetStringLibrary.Conv_StringToInt` (`KismetStringLibrary.GetSubstring` (`KismetSystemLibrary.GetObjectName` (`self.SelectedCable`)) 5)) 2)))
    (:`Socket3`
      (`CableComponent.SetAttachEndToComponent` _selectedcable (`self.Center3`) "None")
      (if (`KismetStringLibrary.EqualEqual_StrStr` (`KismetSystemLibrary.GetObjectName` (`PrimitiveComponent.GetMaterial` (`self.SelectedCable`) 0)) (`KismetSystemLibrary.GetObjectName` (`PrimitiveComponent.GetMaterial` (`self.Socket3`) 0)))
        (`BlueprintMapLibrary.Map_Add` (`self.MapCorrectSocket`) (`KismetStringLibrary.Conv_StringToInt` (`KismetStringLibrary.GetSubstring` (`KismetSystemLibrary.GetObjectName` (`self.SelectedCable`)) 5)) 3)))
    (:`Socket4`
      (`CableComponent.SetAttachEndToComponent` _selectedcable (`self.Center4`) "None")
      (if (`KismetStringLibrary.EqualEqual_StrStr` (`KismetSystemLibrary.GetObjectName` (`PrimitiveComponent.GetMaterial` (`self.SelectedCable`) 0)) (`KismetSystemLibrary.GetObjectName` (`PrimitiveComponent.GetMaterial` (`self.Socket4`) 0)))
        (`BlueprintMapLibrary.Map_Add` (`self.MapCorrectSocket`) (`KismetStringLibrary.Conv_StringToInt` (`KismetStringLibrary.GetSubstring` (`KismetSystemLibrary.GetObjectName` (`self.SelectedCable`)) 5)) 4)))))

(fn `f_GenerateRandomColors`
  (bind _listcolors (`self.ListColors`))
  (for (_ _array_index) _listcolors
    (`KismetArrayLibrary.Array_Swap` _listcolors _array_index (`KismetMathLibrary.RandomInteger` 4)))
  (for _ _listcolors
    _))

(fn `f_RandomCable`
  (params (Selection :type Integer) (`Dimension 1` :type Integer))
  (bind _output (`|GetArrayItem` (`self.ListCables`) `Dimension 1`))
  (switch `int` Selection
    (:`1`
      (`/Engine/EditorBlueprintResources/StandardMacros.IsValid` _output
        (:`Is Valid`
          (`PrimitiveComponent.SetMaterial` _output 0 "/Game/Material/M_Blue.M_Blue"))))
    (:`2`
      (`/Engine/EditorBlueprintResources/StandardMacros.IsValid` _output
        (:`Is Valid`
          (`PrimitiveComponent.SetMaterial` _output 0 "/Game/Material/M_Red.M_Red"))))
    (:`3`
      (`/Engine/EditorBlueprintResources/StandardMacros.IsValid` _output
        (:`Is Valid`
          (`PrimitiveComponent.SetMaterial` _output 0 "/Game/Material/M_Green.M_Green"))))
    (:`4`
      (`/Engine/EditorBlueprintResources/StandardMacros.IsValid` _output
        (:`Is Valid`
          (`PrimitiveComponent.SetMaterial` _output 0 "/Game/Material/M_Yellow.M_Yellow"))))))

(fn `f_RandomSocket`
  (params (Selection :type Integer) (`Dimension 1` :type Integer))
  (bind _output (`|GetArrayItem` (`self.ListSockets`) `Dimension 1`))
  (switch `int` Selection
    (:`1`
      (`PrimitiveComponent.SetMaterial` _output 0 "/Game/Material/M_Blue.M_Blue"))
    (:`2`
      (`PrimitiveComponent.SetMaterial` _output 0 "/Game/Material/M_Red.M_Red"))
    (:`3`
      (`PrimitiveComponent.SetMaterial` _output 0 "/Game/Material/M_Green.M_Green"))
    (:`4`
      (`PrimitiveComponent.SetMaterial` _output 0 "/Game/Material/M_Yellow.M_Yellow"))))

(fn `f_TakeCable`
  (params (Name :type String))
  (bind _cube1 (`self.Cube1`))
  (bind _cube2 (`self.Cube2`))
  (bind _cube3 (`self.Cube3`))
  (bind _cube4 (`self.Cube4`))
  (bind _returnvalue (`KismetStringLibrary.Conv_StringToInt` (`KismetStringLibrary.GetSubstring` (`KismetSystemLibrary.GetObjectName` (`self.SelectedCable`)) 5)))
  (switch `string` Name
    (:`Cube1`
      (`PrimitiveComponent.SetMaterial` _cube1 0 (`self.Interacting`))
      (set `self.SelectedCube` _cube1)
      (set `self.SelectedCable` (`self.Cable1`)))
    (:`Cube2`
      (`PrimitiveComponent.SetMaterial` _cube2 0 (`self.Interacting`))
      (set `self.SelectedCube` _cube2)
      (set `self.SelectedCable` (`self.Cable2`)))
    (:`Cube3`
      (`PrimitiveComponent.SetMaterial` _cube3 0 (`self.Interacting`))
      (set `self.SelectedCube` _cube3)
      (set `self.SelectedCable` (`self.Cable3`)))
    (:`Cube4`
      (`PrimitiveComponent.SetMaterial` _cube4 0 (`self.Interacting`))
      (set `self.SelectedCube` _cube4)
      (set `self.SelectedCable` (`self.Cable4`))))
  (if (`BlueprintMapLibrary.Map_Contains` (`self.MapCorrectSocket`) _returnvalue)
    (`BlueprintMapLibrary.Map_Remove` (`self.MapCorrectSocket`) _returnvalue)))

(fn `UserConstructionScript`)