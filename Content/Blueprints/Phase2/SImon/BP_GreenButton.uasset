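; BP_GreenButton is the green input button for a Simon memory game managed by BP_Simon, which it looks up at BeginPlay.
; When the player character overlaps its collision while Simon allows interaction, it locks interaction and swaps Simon's green mesh to a lit material for a short delay.
; It then restores the material, re-enables interaction and passes the green index to Simon's VerifyRespond to check the answer.
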(event `self.ReceiveBeginPlay`
  (bind _returnvalue (`GameplayStatics.GetActorOfClass` "/Game/Blueprints/Phase2/SImon/BP_Simon.BP_Simon_C"))
  (set `self.Simon` _returnvalue))

(event `self.collision.OnComponentBeginOverlap`
  (params (OverlappedComponent :type "PrimitiveComponent Object Reference") (OtherActor :type "Actor Object Reference") (OtherComp :type "PrimitiveComponent Object Reference") (OtherBodyIndex :type Integer) (bFromSweep :type Boolean) (SweepResult :type "HitResult Structure (by ref)"))
  (bind _simon (`self.Simon`))
  (bind _green (`/Game/Blueprints/Phase2/SImon/BP_Simon.Green` (`self.Simon`)))
  (if (`/Game/Blueprints/Phase2/SImon/BP_Simon.CanInteract` (`self.Simon`))
    (if (== OtherActor (`GameplayStatics.GetPlayerCharacter` 0))
      (`KismetSystemLibrary.PrintString` "green")
      (set `/Game/Blueprints/Phase2/SImon/BP_Simon.CanInteract` false (`self.Simon`))
      (`PrimitiveComponent.SetMaterial` _green 0 "/Game/Material/M_GreenLight.M_GreenLight")
      (`KismetSystemLibrary.Delay` 1.5)
      (`PrimitiveComponent.SetMaterial` _green 0 "/Game/Material/M_Green.M_Green")
      (set `/Game/Blueprints/Phase2/SImon/BP_Simon.CanInteract` true _simon)
      (`/Game/Blueprints/Phase2/SImon/BP_Simon.VerifyRespond` _simon 2))))

(fn `UserConstructionScript`)