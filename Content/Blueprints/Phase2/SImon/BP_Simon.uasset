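; Simon-style color memory game actor with Blue, Red, Yellow and Green components.
; On BeginPlay it randomizes List entries and swaps the matching color's material, then again after a 1.2-second Delay inside the loop.
; CustomEvent chains debug-printed checks: Blue by material name, then Yellow and Green by material slot-name validity, setting OK flags.
; Red is never checked, and no player input is handled here.
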(event `CustomEvent`
  ;[1 1 1] Blue OK
  (`KismetSystemLibrary.PrintString` "modele fini")
  (if (`KismetStringLibrary.EqualEqual_StrStr` (`KismetSystemLibrary.GetObjectName` (`PrimitiveComponent.GetMaterial` (`self.Blue`) 0)) "M_BlueLight")
    (set `self.BlueOK` true)
    ;[1 1 1] Yellow OK
    (`KismetSystemLibrary.PrintString` "blueOK")
    (if (`MeshComponent.IsMaterialSlotNameValid` (`self.Yellow`) "M_YellowLight")
      (set `self.YellowOK` true)
      ;[1 1 1] Green OK
      (`KismetSystemLibrary.PrintString` "yellowOK")
      (if (`MeshComponent.IsMaterialSlotNameValid` (`self.Green`) "M_GreenLight")
        (set `self.GreenOK` true)
        (else
          (set `self.GreenOK` false)
          (`KismetSystemLibrary.PrintString` "NO GREEN")))
      (else
        (set `self.YellowOK` false)
        (`KismetSystemLibrary.PrintString` "NO YELLOW")))
    (else
      (set `self.BlueOK` false)
      (`KismetSystemLibrary.PrintString` "NO BLUE"))))

(event `self.ReceiveBeginPlay`
  (bind _blue (`self.Blue`))
  (bind _red (`self.Red`))
  (bind _yellow (`self.Yellow`))
  (bind _green (`self.Green`))
  (bind _list (`self.List`))
  (for (_array_element _array_index) _list
    (`KismetArrayLibrary.Array_Set` _list _array_index (`KismetMathLibrary.RandomInteger` 3))
    (if (== _array_element (`self.BlueValue`))
      (`PrimitiveComponent.SetMaterial` _blue 0 null)
      (`KismetSystemLibrary.Delay` 1.2)
      (`PrimitiveComponent.SetMaterial` _blue 0 null)
      (elif (== _array_element (`self.RedValue`))
        (`PrimitiveComponent.SetMaterial` _red 0 null)
        (`KismetSystemLibrary.Delay` 1.2)
        (`PrimitiveComponent.SetMaterial` _red 0 null)
        (elif (== _array_element (`self.YellowValue`))
          (`PrimitiveComponent.SetMaterial` _yellow 0 null)
          (`KismetSystemLibrary.Delay` 1.2)
          (`PrimitiveComponent.SetMaterial` _yellow 0 null)
          (elif (== _array_element (`self.GreenValue`))
            (`PrimitiveComponent.SetMaterial` _green 0 null)
            (`KismetSystemLibrary.Delay` 1.2)
            (`PrimitiveComponent.SetMaterial` _green 0 null)))))))

(fn `UserConstructionScript`)