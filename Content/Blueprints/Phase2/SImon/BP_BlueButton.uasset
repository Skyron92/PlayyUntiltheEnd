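; Blue input button for the Simon color-sequence game, triggered when the player character overlaps its collision.
; It finds the BP_Simon actor on BeginPlay and responds only while that actor's CanInteract flag is true.
; A press locks interaction and briefly lights Simon's blue component through a material swap.
; After a delay it restores the material, unlocks interaction and reports the blue index to Simon's VerifyRespond.
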(event `self.ReceiveBeginPlay`
  (bind _returnvalue (`GameplayStatics.GetActorOfClass` "/Game/Blueprints/Phase2/SImon/BP_Simon.BP_Simon_C"))
  (set `self.Simon` _returnvalue))

(event `self.collision.OnComponentBeginOverlap`
  (params (OverlappedComponent :type "PrimitiveComponent Object Reference") (OtherActor :type "Actor Object Reference") (OtherComp :type "PrimitiveComponent Object Reference") (OtherBodyIndex :type Integer) (bFromSweep :type Boolean) (SweepResult :type "HitResult Structure (by ref)"))
  (bind _simon (`self.Simon`))
  (bind _simon_2 (`self.Simon`))
  (bind _blue (`/Game/Blueprints/Phase2/SImon/BP_Simon.Blue` _simon))
  (if (`/Game/Blueprints/Phase2/SImon/BP_Simon.CanInteract` (`self.Simon`))
    (if (== OtherActor (`GameplayStatics.GetPlayerCharacter` 0))
      (`KismetSystemLibrary.PrintString` "blue")
      (set `/Game/Blueprints/Phase2/SImon/BP_Simon.CanInteract` false _simon)
      (`PrimitiveComponent.SetMaterial` _blue 0 "/Game/Material/M_BlueLight.M_BlueLight")
      (`KismetSystemLibrary.Delay` 1.5)
      (`PrimitiveComponent.SetMaterial` _blue 0 "/Game/Material/M_Blue.M_Blue")
      (set `/Game/Blueprints/Phase2/SImon/BP_Simon.CanInteract` true _simon_2)
      (`/Game/Blueprints/Phase2/SImon/BP_Simon.VerifyRespond` _simon_2 0))))

(fn `UserConstructionScript`)