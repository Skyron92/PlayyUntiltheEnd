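; Obstacle actor that moves along negative world Y while the game runs, tracked by an obstacle manager.
; Each Tick, unless IsPaused is set, it offsets itself by the negated product of BaseSpeed and Speed, without delta-time scaling.
; On destruction, a handler bound at BeginPlay removes it from the InstanceList of ObstacleManagerRef.
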(event `self.ReceiveTick`
  (params (DeltaSeconds :type "Float (single-precision)"))
  (bind _returnvalue (* (`self.BaseSpeed`) (`self.Speed`)))
  (if (not (`self.isPaused`))
    (`self.K2_AddActorWorldOffset` (`KismetMathLibrary.MakeVector` 0.0 (- _returnvalue (* _returnvalue 2.0))))))

(event `self.ReceiveBeginPlay`
  (add `self.OnDestroyed` (delegate `OnDestroyed_Event`)))

(event `OnDestroyed_Event` :!signature `self.OnDestroyed`
  (params (DestroyedActor :type "Actor Object Reference"))
  (`KismetArrayLibrary.Array_RemoveItem` (`/Game/Blueprints/Phase1/BP_ObstaclesManager.InstanceList` (`self.ObstacleManagerRef`)) self))

(fn `UserConstructionScript`)