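; Obstacle spawner for a minigame: periodically spawns a random obstacle at a start point and passes it a manager reference and speed.
; A Delay on Tick paces spawning, with a random interval that shrinks as the GameInstance's finished-minigame count rises.
; A Box overlap destroys incoming actors and adds bonus time to the GameInstance every tenth one.
; Pause functions halt spawning and flag tracked instances, saving and restoring speed.
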(event `self.ReceiveBeginPlay`
  (set `self.StartPoint` (`SceneComponent.K2_GetComponentLocation` (`self.StartPointObject`)))
  (set `self.spawnDuration` 1.0))

(event `self.ReceiveTick`
  (params (DeltaSeconds :type "Float (single-precision)"))
  (bind _obstacleslist (`self.ObstaclesList`))
  (`KismetSystemLibrary.Delay` (`self.spawnDuration`))
  (if (not (`self.isPaused`))
    (bind _returnvalue (`|SpawnActorFromClass` (`GameplayStatics.GetObjectClass` (`|GetArrayItem` _obstacleslist (`KismetMathLibrary.RandomInteger` (`KismetArrayLibrary.Array_Length` _obstacleslist)))) (`KismetMathLibrary.MakeTransform` (`self.StartPoint`) (struct :`Yaw` 90.0) (0.05 0.05 0.05)) "Undefined" "MultiplyWithRoot" null null))
    (`KismetArrayLibrary.Array_Add` (`self.InstanceList`) _returnvalue)
    (set `/Game/Blueprints/Phase1/Enemy/BP_Enemy.ObstacleManager` self _returnvalue)
    (set `/Game/Blueprints/Phase1/Enemy/BP_Enemy.Speed` (`self.speedManager`) _returnvalue)
    (set `self.spawnDuration` (- (`KismetMathLibrary.RandomFloatInRange` 0.8 1.0) (* (/ (`/Game/Blueprints/Quest/BP_GameInstance.MiniGameFinished` (cast `/Game/Blueprints/Quest/BP_GameInstance` (`GameplayStatics.GetGameInstance`) :!pure true)) 2) 0.05)))))

(event `self.Box.OnComponentBeginOverlap`
  (params (OverlappedComponent :type "PrimitiveComponent Object Reference") (OtherActor :type "Actor Object Reference") (OtherComp :type "PrimitiveComponent Object Reference") (OtherBodyIndex :type Integer) (bFromSweep :type Boolean) (SweepResult :type "HitResult Structure (by ref)"))
  (bind _counter (`self.Counter`))
  (bind _asbp_game_instance (cast `/Game/Blueprints/Quest/BP_GameInstance` (`GameplayStatics.GetGameInstance`) :!pure true))
  (`self.K2_DestroyActor` OtherActor)
  (`/Engine/EditorBlueprintResources/StandardMacros.IncrementInt` _counter
    (:`  `
      (if (== _counter 10)
        (set `/Game/Blueprints/Quest/BP_GameInstance.Time` (+ (`/Game/Blueprints/Quest/BP_GameInstance.Time` _asbp_game_instance) 5.0) _asbp_game_instance)
        (set `self.Counter` 0)))))

(fn `PauseGame`
  (set `self.speedPauseReference` (`self.speedManager`))
  (set `self.speedManager` 0.0)
  (set `self.isPaused` true)
  (for _array_element (`self.InstanceList`)
    (set `/Game/Blueprints/Phase1/Enemy/BP_Enemy.isPaused` true _array_element)))

(fn `UnpauseGame`
  (set `self.speedManager` (`self.speedPauseReference`))
  (set `self.isPaused` false)
  (for _array_element (`self.InstanceList`)
    (set `/Game/Blueprints/Phase1/Enemy/BP_Enemy.isPaused` false _array_element)))

(fn `UserConstructionScript`)