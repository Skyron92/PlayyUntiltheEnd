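; BP_Enemy is a Phase 1 enemy actor that travels along negative Y and is tracked by an obstacle manager.
; Each Tick steps its location by a speed that rises with the game instance's MiniGameFinished value, without delta-time scaling.
; When IsPaused is set it destroys itself rather than halting, and its OnDestroyed handler removes it from the ObstacleManager's InstanceList.
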(event `self.ReceiveTick`
  (params (DeltaSeconds :type "Float (single-precision)"))
  (bind (_returnvalue_x _returnvalue_y _returnvalue_z) (`KismetMathLibrary.BreakVector` (`self.K2_GetActorLocation`)))
  (if (`self.isPaused`)
    (`self.K2_DestroyActor`)
    (else
      (`self.K2_SetActorLocation` (`KismetMathLibrary.MakeVector` _returnvalue_x (+ _returnvalue_y (* (* (+ (`self.BaseSpeed`) (* (`/Game/Blueprints/Quest/BP_GameInstance.MiniGameFinished` (cast `/Game/Blueprints/Quest/BP_GameInstance` (`GameplayStatics.GetGameInstance`) :!pure true)) 0.025)) (`self.Speed`)) -1.0)) _returnvalue_z)))))

(event `self.ReceiveBeginPlay`
  (add `self.OnDestroyed` (delegate `OnDestroyed_Event`)))

(event `OnDestroyed_Event` :!signature `self.OnDestroyed`
  (params (DestroyedActor :type "Actor Object Reference"))
  (`KismetArrayLibrary.Array_RemoveItem` (`/Game/Blueprints/Phase1/BP_ObstaclesManager.InstanceList` (`self.ObstacleManager`)) self))

(fn `UserConstructionScript`)