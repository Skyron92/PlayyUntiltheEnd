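; BP_PlatformerCharacter is the player-controlled platformer character, with a jump gated by a custom grounded flag.
; On BeginPlay it has its controller possess it and adds the default Enhanced Input mapping context.
; Overlapping a BP_StartPointCharacter sets IsGrounded and leaving clears it; the jump action only jumps while that flag is set.
; Debug prints remain on input and startup, alongside disconnected position and pause-check nodes.
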(event `self.ReceiveBeginPlay`
  (bind _returnvalue (`self.GetController`))
  (bind _asplayer_controller (cast `PlayerController` _returnvalue))
  (`Controller.Possess` _returnvalue self)
  (bind _returnvalue_2 (pcsubsystem `EnhancedInputLocalPlayerSubsystem` _asplayer_controller))
  (`/Engine/EditorBlueprintResources/StandardMacros.IsValid` _returnvalue_2
    (:`Is Valid`
      (`EnhancedInputSubsystemInterface.AddMappingContext` _returnvalue_2 "/Game/FirstPerson/Input/IMC_Default.IMC_Default" 0 (struct))
      (`KismetSystemLibrary.PrintString` (`KismetSystemLibrary.GetDisplayName` _asplayer_controller))
      (bind _output_get (set `self.StartLocation` (0.0 0.0 0.0))))))

(event `EnhancedInput|/Game/FirstPerson/Input/Actions/IA_Jump`
  (params (ActionValue :type Boolean) (ElapsedSeconds :type "Float (double-precision)") (TriggeredSeconds :type "Float (double-precision)") (InputAction :type "InputAction Object Reference" :default "/Game/FirstPerson/Input/Actions/IA_Jump.IA_Jump"))
  (:`Triggered`
    (`KismetSystemLibrary.PrintString` "Hello" :!label _label)
    (if (`self.IsGrounded`)
      (`KismetSystemLibrary.PrintString` "Hello")
      (`self.Jump`)))
  (:`Started`
    (goto _label))
  (:`Ongoing`
    (goto _label)))

(event `self.ReceiveActorBeginOverlap`
  (params (OtherActor :type "Actor Object Reference"))
  (cast `/Game/Blueprints/Phase1/BP_StartPointCharacter` OtherActor)
  (set `self.IsGrounded` true))

(event `self.ReceiveActorEndOverlap`
  (params (OtherActor :type "Actor Object Reference"))
  (cast `/Game/Blueprints/Phase1/BP_StartPointCharacter` OtherActor)
  (set `self.IsGrounded` false))

(event `Key|Z`
  (params (Key :type "Key Structure"))
  (:`Pressed`
    (`KismetSystemLibrary.PrintString` "Hello")))

(event `self.ReceiveTick`
  (params (DeltaSeconds :type "Float (single-precision)")))

(fn `UserConstructionScript`)